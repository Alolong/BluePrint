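; BP_MoveRect is an actor that moves its Cube along a rectangular path in the local X-Z plane while enabled.
; Tick switches on the PlusMinus direction state, stepping Xmove or Zmove by a fixed per-frame amount, independent of delta time, and applying the relative location.
; Reaching a bound changes the state to turn onto the other axis.
; OverlapAction sets the Isplay flag that gates the movement.
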(event EventTick
  (params (DeltaSeconds :type Float%20%28single-precision%29))
  (if (Variables|Default|Getisplay)
    (switch Utilities|FlowControl|Switch|SwitchonEM_MoveSelect (Variables|Default|GetPlusMinus)
      (:NewEnumerator0
        ;[0.15 0.15 0.15 0.5] X+
        (bind _output_get (Variables|Default|SetXmove (+ (Variables|Default|GetXmove) 5.0)))
        (Transformation|SetRelativeLocation (Variables|Default|GetCube) (Math|Vector|MakeVector _output_get 0.0 (Variables|Default|GetZmove)) false false)
        (if (>= (Variables|Default|GetXmove) 1e+02)
          (Variables|Default|SetPlusMinus "NewEnumerator1")))
      (:NewEnumerator1
        ;[0.15 0.15 0.15 0.5] Z+
        (bind _output_get_2 (Variables|Default|SetZmove (+ (Variables|Default|GetZmove) 5.0)))
        (Transformation|SetRelativeLocation (Variables|Default|GetCube) (Math|Vector|MakeVector (Variables|Default|GetXmove) 0.0 _output_get_2) false false)
        (if (>= (Variables|Default|GetZmove) 1e+02)
          (Variables|Default|SetPlusMinus "NewEnumerator2")))
      (:NewEnumerator2
        ;[0.15 0.15 0.15 0.5] -X
        (bind _output_get_3 (Variables|Default|SetXmove (- (Variables|Default|GetXmove) 5.0)))
        (Transformation|SetRelativeLocation (Variables|Default|GetCube) (Math|Vector|MakeVector _output_get_3 0.0 (Variables|Default|GetZmove)) false false)
        (if (<= (Variables|Default|GetXmove) 0.0)
          (Variables|Default|SetPlusMinus "NewEnumerator3")))
      (:NewEnumerator3
        ;[0.15 0.15 0.15 0.5] Z-
        (bind _output_get_4 (Variables|Default|SetZmove (- (Variables|Default|GetZmove) 5.0)))
        (Transformation|SetRelativeLocation (Variables|Default|GetCube) (Math|Vector|MakeVector (Variables|Default|GetXmove) 0.0 _output_get_4) false false)
        (if (<= (Variables|Default|GetZmove) 0.0)
          (Variables|Default|SetPlusMinus "NewEnumerator0"))))))

(fn ConstructionScript)

(fn OverlapAction
  (params (come :type Boolean))
  (Variables|Default|Setisplay come)
  (return false))