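; BP_Timer is a play timer that shows elapsed time on the HUD.
; OverlapAction switches counting on or off through its Come argument and always returns false.
; While running, Tick accumulates delta seconds, uses Floor00 to zero-pad minutes and seconds, and sends the minutes:seconds string to BP_Hud's CountTime through player controller 0.
; The count is never reset here, so stopping only pauses it.
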(event EventTick
  (params (DeltaSeconds :type Float%20%28single-precision%29))
  (if (Variables|Default|Getisplay)
    (bind _output_get (Variables|Default|SetCount (+ DeltaSeconds (Variables|Default|GetCount))))
    (bind _asbp_hud (Utilities|Casting|CastToBP_Hud (HUD|GetHUD (Game|GetPlayerController 0))))
    (Default|CountTime _asbp_hud (Utilities|String|Append (CallFunction|Floor00 (/ _output_get 6e+01)) ":" (CallFunction|Floor00 (Math|Float|%(Float) _output_get 6e+01))))))

(fn ConstructionScript)

(fn Floor00
  (params (A :type Float%20%28double-precision%29))
  (bind _returnvalue (Math|Float|Floor A))
  (if (< A 1e+01)
    (return (Utilities|String|Append "0" (Utilities|String|ToString(Integer) _returnvalue)))
    (else
      (return (Utilities|String|ToString(Integer) _returnvalue)))))

(fn OverlapAction
  (params (come :type Boolean))
  (Variables|Default|Setisplay come)
  (return false))