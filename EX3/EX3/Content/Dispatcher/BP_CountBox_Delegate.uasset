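; BP_CountBox_Delegate is a counter box that shows a cycling count on a widget, driven by an event dispatcher.
; On BeginPlay it binds an event to its Switch reference, and the countbox event increments Count and passes it to the BP_count widget.
; After displaying 9, Count resets to -1 so the next increment shows 0.
; OverlapAction stores its Come input in Isplay and returns false.
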(event Custom|countbox
  (Variables|Default|Setcount (+ (Variables|Default|Getcount) 1))
  (bind _asbp_count (Utilities|Casting|CastToBP_count (UserInterface|GetWidget (Variables|Default|GetWidget))))
  (Default|CountBox _asbp_count (Variables|Default|Getcount))
  (if (== (Variables|Default|Getcount) 9)
    (Variables|Default|Setcount -1)))

(event EventBeginPlay
  (EventDispatchers|BindEventtoDispatcher (Variables|Default|Getswitch) (EventDispatchers|CreateEvent :!event BPCountBoxDelegateAutoGenFunc)))

(fn ConstructionScript)

(fn BPCountBoxDelegateAutoGenFunc
  (params (begin :type Boolean))
  (CallFunction|Countbox))

(fn OverlapAction
  (params (come :type Boolean))
  (Variables|Default|Setisplay come)
  (return false))