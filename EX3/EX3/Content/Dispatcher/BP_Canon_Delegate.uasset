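; Cannon actor that fires bullets repeatedly, controlled by a switch through an event dispatcher.
; On BeginPlay it binds to the Switch's dispatcher, and a Begin-flag function chooses between Doplay and DoStop.
; Doplay fires immediately and starts a looping Doshot timer, spawning BP_bullet_Delegate at component R with Shootspeed as impulse.
; DoStop calls the timer clear with an empty function name, so it does not target Doshot.
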(event Custom|Do%20play
  (Utilities|Time|SetTimerbyFunctionName 0 "Doshot" 1.0 true)
  (CallFunction|Doshot))

(event Custom|Do%20Stop
  (Utilities|Time|ClearTimerbyFunctionName 0 ""))

(event Custom|Doshot
  (bind _r (Variables|Default|Getr))
  (bind _returnvalue (Transformation|GetWorldTransform _r))
  (Game|SpawnActorfromClass "/Game/Dispatcher/BP_bullet_Delegate.BP_bullet_Delegate_C" (Math|Transform|MakeTransform (.location _returnvalue) (.rotation _returnvalue) "1.000000,1.000000,1.000000") "Undefined" "MultiplyWithRoot" 0 (Variables|Default|Getshootspeed) 0))

(event EventBeginPlay
  (EventDispatchers|BindEventtoDispatcher (Variables|Default|Getswitch) (EventDispatchers|CreateEvent :!event BPCanonDelegateAutoGenFunc)))

(event Collision|EventActorBeginOverlap
  (params (OtherActor :type Actor%20Object%20Reference)))

(event EventTick
  (params (DeltaSeconds :type Float%20%28single-precision%29)))

(fn ConstructionScript)

(fn BPCanonDelegateAutoGenFunc
  (params (begin :type Boolean))
  (if begin
    (CallFunction|DoPlay)
    (else
      (CallFunction|DoStop))))