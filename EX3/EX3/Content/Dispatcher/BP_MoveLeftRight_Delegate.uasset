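; Dispatcher-driven actor that slides its Cube back and forth along relative X while a play flag is on.
; On BeginPlay it binds a created event to the event dispatcher on its Switch reference; handler functions set the play flag from a boolean.
; Tick steps the X offset by a fixed, frame-rate-dependent amount, flipping direction at each end of the range.
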(event EventBeginPlay
  (EventDispatchers|BindEventtoDispatcher (Variables|Default|Getswitch) (EventDispatchers|CreateEvent :!event BPMoveLeftRightDelegateAutoGenFunc)))

(event EventTick
  (params (DeltaSeconds :type Float%20%28single-precision%29))
  (if (Variables|Default|Getisplay)
    (if (Variables|Default|GetPlusMinus)
      ;[0.15 0.15 0.15 0.5] X+
      (bind _output_get (Variables|Default|SetXmove (+ (Variables|Default|GetXmove) 5.0)))
      (Transformation|SetRelativeLocation (Variables|Default|GetCube) (Math|Vector|MakeVector _output_get 0.0 0.0) false false)
      (if (>= (Variables|Default|GetXmove) 1e+02)
        (Variables|Default|SetPlusMinus false))
      (else
        ;[0.15 0.15 0.15 0.5] -X
        (bind _output_get_2 (Variables|Default|SetXmove (- (Variables|Default|GetXmove) 5.0)))
        (Transformation|SetRelativeLocation (Variables|Default|GetCube) (Math|Vector|MakeVector _output_get_2 0.0 0.0) false false)
        (if (<= (Variables|Default|GetXmove) 0.0)
          (Variables|Default|SetPlusMinus true))))))

(fn ConstructionScript)

(fn BPMoveLeftRightDelegateAutoGenFunc
  (params (begin :type Boolean))
  (Variables|Default|Setisplay begin))

(fn OverlapAction
  (params (come :type Boolean))
  (Variables|Default|Setisplay come)
  (return false))