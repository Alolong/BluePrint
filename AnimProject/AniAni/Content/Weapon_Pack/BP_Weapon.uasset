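; BP_Weapon is a melee weapon actor that attaches to a character's Sword socket and deals damage along its mesh.
; DoAttach stores the wielding character and snaps the weapon onto that character's skeletal mesh, keeping world scale.
; DoDamage box-traces between the mesh's HitA and HitB sockets, ignoring the wielder.
; It applies fixed damage credited to the wielder's controller, returning after the first hit.
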(event EventBeginPlay)

(event Collision|EventActorBeginOverlap
  (params (OtherActor :type Actor%20Object%20Reference)))

(event EventTick
  (params (DeltaSeconds :type Float%20%28single-precision%29)))

(fn ConstructionScript)

(fn DoAttach
  (params (Character :type Character%20Object%20Reference))
  (bind _output_get (Variables|Default|SetCharacter Character))
  (Transformation|AttachComponentToComponent (Variables|/Script/Engine.Character|GetMesh _output_get) "Sword" "SnapToTarget" "SnapToTarget" "KeepWorld" true))

(fn DoDamage
  (bind _staticmesh (Variables|Default|GetStaticMesh))
  ;[0.15 0.15 0.15 0.5] 멀티박스 트레이스- 궤적을 박스로
  (bind _outhits (Class|KismetSystemLibrary|BoxTraceMultiforObjects (Transformation|GetSocketLocation _staticmesh "HitA") (Transformation|GetSocketLocation _staticmesh "HitB") "1.000000,1.000000,1.000000" "0, 0, 0" (Utilities|Array|MakeArray "ObjectTypeQuery3" "ObjectTypeQuery5" "ObjectTypeQuery6" "ObjectTypeQuery1" "ObjectTypeQuery2") false (Utilities|Array|MakeArray (Variables|Default|GetCharacter)) "None" true))
  (for _array_element _outhits
    (Game|Damage|ApplyDamage (.HitActor (Collision|BreakHitResult _array_element)) 1.2e+02 (Pawn|GetController (Variables|Default|GetCharacter)) self)
    (return false)))