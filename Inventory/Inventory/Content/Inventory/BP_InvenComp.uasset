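; Inventory component that manages a fixed array of item slots, created on BeginPlay and filled with the "Empty" row from DT_Item.
; AddItem copies a DT_Item row into the first empty slot without checking IsFull, RemoveItem resets a slot to Empty, and SwapItem exchanges two slots.
; Changes call the DSCahngeInven dispatcher, and add and remove also print every slot for debugging.
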(event EventBeginPlay
  (CallFunction|CreateInvenSlot 10))

(event EventTick
  (params (DeltaSeconds :type Float%20%28single-precision%29)))

(fn AddItem
  (params (RowName :type Name))
  ;[0.15 0.15 0.15 0.5] 오버랩-아이템베이스-변수
  ; ThirdPerson-각 아이템 1,2,3
  ;[0.15 0.15 0.15 0.5] Empty가 아닐 경우만 아이템을 넣어라
  (if (!= RowName "Empty")
    ;[0.15 0.15 0.15 0.5] 빈 슬롯 찾기 함수
    (bind _returnvalue (Utilities|GetDataTableRow "/Game/Inventory/Items/DT_Item.DT_Item" RowName)
      (:then
        (bind _index (CallFunction|FindEmptySlot))
        ;[0.15 0.15 0.15 0.5] 대상을 슬롯에 Set
        ;;[0.15 0.15 0.15 0.5] split pin
        (Utilities|Array|SetArrayElem (Variables|Default|GetSlot) _index (Utilities|Struct|MakeST_ItemSlot 1 _returnvalue))
        (CallFunction|PrintAllSlot)
        (Default|CallDSCahngeInven)))))

(fn RemoveItem
  (params (Index :type Integer))
  ;[0.15 0.15 0.15 0.5] 캐릭터에서만
  (CallFunction|SetEmptySlot Index)
  (CallFunction|PrintAllSlot)
  (Default|CallDSCahngeInven))

(fn SwapItem
  (params (From :type Integer) (To :type Integer))
  ;[0.15 0.15 0.15 0.5] 아이템의 자리 바꾸기: 위젯 사용
  (Utilities|Array|Swap (Variables|Default|GetSlot) From To)
  (Default|CallDSCahngeInven))

(fn CreateInvenSlot
  (params (Count :type Integer))
  ;[0.15 0.15 0.15 0.5] 배열의 전체 각각0 부터 9
  (for _index (range 0 (- Count 1))
    ;[0.15 0.15 0.15 0.5] 데이터 테이블 배열 생성
    (bind _returnvalue (Utilities|GetDataTableRow "/Game/Inventory/Items/DT_Item.DT_Item" "Empty")
      (:then
        (Utilities|Array|Add (Variables|Default|GetSlot) (Utilities|Struct|MakeST_ItemSlot _index _returnvalue))))))

(fn IsEmptySlot
  (params (Index :type Integer))
  (return (Utilities|Enum|Equal(Enum) (.name (.ItemData (Utilities|Struct|BreakST_ItemSlot (Utilities|Array|Get(acopy) (Variables|Default|GetSlot) Index)))) "Empty")))

(fn SetEmptySlot
  (params (Index :type Integer))
  (bind _returnvalue (Utilities|GetDataTableRow "/Game/Inventory/Items/DT_Item.DT_Item" "Empty")
    (:then
      ;[0.15 0.15 0.15 0.5] ItemData활성화(details)
      (Utilities|Struct|SetmembersinST_ItemSlot (Utilities|Array|Get(acopy) (Variables|Default|GetSlot) Index) _returnvalue)
      (Default|CallDSCahngeInven))))

(fn FindEmptySlot
  ;[0.15 0.15 0.15 0.5] 전체 배열 체크
  (for (_ _array_index) (Variables|Default|GetSlot)
    ;[0.15 0.15 0.15 0.5] 빈자리 확인
    (if (CallFunction|IsEmptySlot _array_index)
      ;[0.15 0.15 0.15 0.5] 배열이 다 안참
      (return _array_index false)))
  ;[0.15 0.15 0.15 0.5] 배열이 다참
  (return -1 true))

(fn PrintAllSlot
  (for (_array_element _array_index) (Variables|Default|GetSlot)
    (Development|PrintString (Utilities|String|Append "Index" (Utilities|String|ToString(Integer) _array_index) "Name" (.name (.ItemData (Utilities|Struct|BreakST_ItemSlot _array_element)))) true true "(R=0.000000,G=0.660000,B=1.000000,A=1.000000)" 3.0)))