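; BP_PlayerState tracks the player's coin count and health, and broadcasts changes through event dispatchers.
; GetCoin increments the coin total and sends it out.
; AddDamage and AddHeal act only while the player is alive, report current and max HP, and fire a death dispatcher when HP falls to zero or below.
; Healing clamps to a hard-coded 100 rather than MaxHP, while damage is unclamped.
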(event EventBeginPlay)

(fn ConstructionScript)

(fn GetCoin
  (bind _output_get (Variables|Default|SetCoiin (+ (Variables|Default|GetCoiin) 1)))
  (Default|CallDSCoinGet _output_get))

(fn AddDamage
  (params (Damage :type Float%20%28double-precision%29))
  (if (not (CallFunction|IsDead))
    (bind _output_get (Variables|Default|SetCurHP (- (Variables|Default|GetCurHP) Damage)))
    (Default|CallDSUpdatePlayerHP _output_get (Variables|Default|GetMaxHP))
    (if (CallFunction|IsDead)
      (Default|CallDSDeath))))

(fn IsDead
  (return (<= (Variables|Default|GetCurHP) 0.0)))

(fn AddHeal
  (params (Heal :type Float%20%28double-precision%29))
  (if (not (CallFunction|IsDead))
    (bind _output_get (Variables|Default|SetCurHP (Math|Float|Clamp(Float) (+ (Variables|Default|GetCurHP) Heal) 0.0 1e+02)))
    (Default|CallDSUpdatePlayerHP _output_get (Variables|Default|GetMaxHP))
    (if (CallFunction|IsDead)
      (Default|CallDSDeath))))