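; BP_GoalPost is a team-assigned goal that registers scoring when a BP_Ball overlaps its box.
; On the server only, it passes its Team to the BP_GSB game state's AddTeamGoal, credits a player, then restarts the ball's position.
; Player credit goes to the opposing team's last player recorded on the ball, through that player's BP_PS.
; The construction script sets the mesh material by team.
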(event OnComponentBeginOverlap(Box)
  (params (OverlappedComponent :type Primitive%20Component%20Object%20Reference) (OtherActor :type Actor%20Object%20Reference) (OtherComp :type Primitive%20Component%20Object%20Reference) (OtherBodyIndex :type Integer) (bFromSweep :type Boolean) (SweepResult :type Hit%20Result%20Structure%20%28by%20ref%29))
  ;[0.15 0.15 0.15 0.5] 서버
  (Networking|SwitchHasAuthority
    (:Authority
      (bind _asbp_ball (Utilities|Casting|CastToBP_Ball OtherActor))
      (bind _asbp_gsb (Utilities|Casting|CastToBP_GSB (Game|GetGameState)))
      (Default|AddTeamGoal _asbp_gsb (Variables|Default|GetTeam))
      (CallFunction|AddPlayerGoal _asbp_ball)
      (Default|ReStartPos _asbp_ball))))

(event EventBeginPlay)

(event Collision|EventActorBeginOverlap
  (params (OtherActor :type Actor%20Object%20Reference)))

(event EventTick
  (params (DeltaSeconds :type Float%20%28single-precision%29)))

(fn ConstructionScript
  (switch Utilities|FlowControl|Switch|SwitchonEN_Team (Variables|Default|GetTeam)
    (:NewEnumerator0
      (Rendering|Material|SetMaterial (Variables|Default|GetStaticMesh) 0 "/Engine/EditorMaterials/WidgetMaterial.WidgetMaterial"))
    (:NewEnumerator1
      (Rendering|Material|SetMaterial (Variables|Default|GetStaticMesh) 0 "/Engine/EditorMaterials/WidgetMaterial_X.WidgetMaterial_X"))
    (:NewEnumerator2
      (Rendering|Material|SetMaterial (Variables|Default|GetStaticMesh) 0 "/Engine/EditorMaterials/WidgetMaterial_Z.WidgetMaterial_Z"))))

(fn AddPlayerGoal
  (params (Ball :type BP%20Ball%20Object%20Reference))
  (switch Utilities|FlowControl|Switch|SwitchonEN_Team (Variables|Default|GetTeam)
    (:NewEnumerator1
      (bind _lastblue (Variables|/Game/BP/BP_Ball.BP_Ball_C|GetLastBlue Ball)
        (:then
          (bind _asbp_ps (Utilities|Casting|CastToBP_PS (Variables|/Script/Engine.Pawn|GetPlayerState _lastblue)))
          (Default|AddGoal _asbp_ps))
        (:else)))
    (:NewEnumerator2
      (bind _lastred (Variables|/Game/BP/BP_Ball.BP_Ball_C|GetLastRed Ball)
        (:then
          (bind _asbp_ps_2 (Utilities|Casting|CastToBP_PS (Variables|/Script/Engine.Pawn|GetPlayerState _lastred)))
          (Default|AddGoal _asbp_ps_2))
        (:else)))))