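; BP_Ball is a physics ball for a team game that remembers the last Red and Blue characters to hit it.
; On the server, sphere hits read the character's team from its BP_PS player state and store that character as LastRed or LastBlue.
; BeginPlay records the start transform on the server, and ReStartPos teleports the ball back there, toggles physics simulation off and on, and clears both records.
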(event OnComponentHit(Sphere)
  (params (HitComponent :type Primitive%20Component%20Object%20Reference) (OtherActor :type Actor%20Object%20Reference) (OtherComp :type Primitive%20Component%20Object%20Reference) (NormalImpulse :type Vector :default "0, 0, 0") (Hit :type Hit%20Result%20Structure%20%28by%20ref%29))
  (Networking|SwitchHasAuthority
    (:Authority
      (bind _ascharacter (Utilities|Casting|CastToCharacter OtherActor))
      (bind _asbp_ps (Utilities|Casting|CastToBP_PS (Variables|/Script/Engine.Pawn|GetPlayerState _ascharacter)))
      (switch Utilities|FlowControl|Switch|SwitchonEN_Team (Variables|/Game/FootBall/GMB/BP_PS.BP_PS_C|GetTeam _asbp_ps)
        (:NewEnumerator1
          (Variables|Default|SetLastRed _ascharacter))
        (:NewEnumerator2
          (Variables|Default|SetLastBlue _ascharacter))))))

(event EventBeginPlay
  (Networking|SwitchHasAuthority
    (:Authority
      (Variables|Default|SetStartBallPos (Transformation|GetActorTransform))
      (CallFunction|ReStartPos))))

(event Collision|EventActorBeginOverlap
  (params (OtherActor :type Actor%20Object%20Reference)))

(event EventTick
  (params (DeltaSeconds :type Float%20%28single-precision%29)))

(fn ConstructionScript)

(fn ReStartPos
  (Transformation|SetActorTransform (Variables|Default|GetStartBallPos) false true)
  (Physics|SetSimulatePhysics (Variables|Default|GetSphere) false)
  (Physics|SetSimulatePhysics (Variables|Default|GetSphere) true)
  (Variables|Default|SetLastRed 0)
  (Variables|Default|SetLastBlue 0))