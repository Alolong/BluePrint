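; BP_GSB is the football game state, tracking match phase, elapsed time and Red and Blue goals.
; Tick accumulates time during Ready and Start, and ChangeGameState resets that timer on each phase switch.
; RepNotify handlers pass score, phase and time changes to event dispatchers.
; AddTeamGoal credits the team opposite the one passed in, GetReult derives a team's outcome from the score, and UpdateResult only casts the game state.
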(event EventTick
  (params (DeltaSeconds :type Float%20%28single-precision%29))
  (switch Utilities|FlowControl|Switch|SwitchonEN_GS (Variables|Default|GetGs)
    (:NewEnumerator1
      (CallFunction|TickReady DeltaSeconds))
    (:NewEnumerator2
      (CallFunction|TickPlay DeltaSeconds))))

(fn ConstructionScript)

(fn AddTeamGoal
  (params (Team :type EN_Team%20Enum :default "NewEnumerator0"))
  (switch Utilities|FlowControl|Switch|SwitchonEN_Team Team
    (:NewEnumerator1
      (Variables|Default|SetBlueGoal (+ (Variables|Default|GetBlueGoal) 1)))
    (:NewEnumerator2
      (Variables|Default|SetRedGoal (+ (Variables|Default|GetRedGoal) 1)))))

(fn OnRepRedGoal
  (Default|CallDSChangeTeamScore (Variables|Default|GetRedGoal) (Variables|Default|GetBlueGoal)))

(fn OnRepBlueGoal
  (Default|CallDSChangeTeamScore (Variables|Default|GetRedGoal) (Variables|Default|GetBlueGoal)))

(fn ChangeGameState
  (params (Gs :type EN_GS%20Enum :default "NewEnumerator0"))
  (Variables|Default|SetGs Gs)
  (Variables|Default|SetTotalDeltaSec 0.0))

(fn OnRepGs
  (Default|CallDSChangeGS (Variables|Default|GetGs)))

(fn TickReady
  (params (DeltaSec :type Float%20%28double-precision%29))
  (Variables|Default|SetTotalDeltaSec (+ (Variables|Default|GetTotalDeltaSec) DeltaSec)))

(fn OnRepTotalDeltaSec
  (Default|CallDSTotalDeltasec (Variables|Default|GetTotalDeltaSec)))

(fn TickPlay
  (params (DeltaSec :type Float%20%28double-precision%29))
  (Variables|Default|SetTotalDeltaSec (+ (Variables|Default|GetTotalDeltaSec) DeltaSec)))

(fn UpdateResult
  (Utilities|Casting|CastToBP_GSB (Game|GetGameState)))

(fn GetReult
  (params (Team :type EN_Team%20Enum :default "NewEnumerator0"))
  (if (== (Variables|Default|GetBlueGoal) (Variables|Default|GetRedGoal))
    (return "NewEnumerator3")
    (else
      (switch Utilities|FlowControl|Switch|SwitchonEN_Team Team
        (:NewEnumerator0
          (return "NewEnumerator3"))
        (:NewEnumerator1
          (if (> (Variables|Default|GetRedGoal) (Variables|Default|GetBlueGoal))
            (return "NewEnumerator1")
            (else
              (return "NewEnumerator2"))))
        (:NewEnumerator2
          (if (> (Variables|Default|GetBlueGoal) (Variables|Default|GetRedGoal))
            (return "NewEnumerator1")
            (else
              (return "NewEnumerator2"))))))))