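; Football game mode that assigns teams and drives the match through Ready, Start and End states.
; Each joining player goes to the smaller team (Red on a tie), and Ready begins once two or more player controllers exist.
; It listens to BP_GSB dispatchers for state and elapsed time, advancing states on time thresholds.
; On End, it tells every BP_PS to update its result.
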(event EventBeginPlay
  ;[0.15 0.15 0.15 0.5] GS
  (bind _asbp_gsb (Utilities|Casting|CastToBP_GSB (Game|GetGameState)))
  (EventDispatchers|AssignDSChangeGS _asbp_gsb (EventDispatchers|CreateEvent :!event EvChangeGS))
  (EventDispatchers|BindEventtoDSTotalDeltasec _asbp_gsb (EventDispatchers|CreateEvent :!event EvTotalDeltaSec)))

(event EventHandleStartingNewPlayer
  (params (NewPlayer :type Player%20Controller%20Object%20Reference))
  ;[0.15 0.15 0.15 0.5] PS
  (|CallParentFunction NewPlayer)
  ;[0.15 0.15 0.15 0.5] 팀 정하기
  (bind _asbp_ps (Utilities|Casting|CastToBP_PS (Variables|/Script/Engine.Controller|GetPlayerState NewPlayer)))
  (Default|UpdateTeam _asbp_ps (CallFunction|FindTeam))
  ;[0.15 0.15 0.15 0.5] Comment
  (if (CallFunction|ChecktoReady)
    (bind _asbp_gsb (Utilities|Casting|CastToBP_GSB (Game|GetGameState)))
    (Default|ChangeGameState _asbp_gsb "NewEnumerator1")))

(fn ConstructionScript)

(fn FindTeam
  (bind _outactors (Actor|GetAllActorsOfClass "/Game/FootBall/GMB/BP_PS.BP_PS_C"))
  (for _array_element _outactors
    (switch Utilities|FlowControl|Switch|SwitchonEN_Team (Variables|/Game/FootBall/GMB/BP_PS.BP_PS_C|GetTeam _array_element)
      (:NewEnumerator1
        (Math|Integer|IncrementInt (LocalVariables|GetRedCount)))
      (:NewEnumerator2
        (Math|Integer|IncrementInt (LocalVariables|GetBlueCount)))))
  (if (> (LocalVariables|GetRedCount) (LocalVariables|GetBlueCount))
    (return "NewEnumerator2")
    (else
      (return "NewEnumerator1"))))

(fn EvChangeGS
  (params (UpdateGS :type EN_GS%20Enum :default "NewEnumerator0"))
  (Variables|Default|SetGS UpdateGS))

(fn EvTotalDeltaSec
  (params (TotalDeltasec :type Float%20%28double-precision%29))
  (switch Utilities|FlowControl|Switch|SwitchonEN_GS (Variables|Default|GetGS)
    (:NewEnumerator1
      (if (> TotalDeltasec 5.0)
        (bind _asbp_gsb (Utilities|Casting|CastToBP_GSB (Game|GetGameState)))
        (Default|ChangeGameState _asbp_gsb "NewEnumerator2")))
    (:NewEnumerator2
      (if (> TotalDeltasec 3e+01)
        (bind _asbp_gsb_2 (Utilities|Casting|CastToBP_GSB (Game|GetGameState)))
        (Default|ChangeGameState _asbp_gsb_2 "NewEnumerator3")
        (bind _outactors (Actor|GetAllActorsOfClass "/Game/FootBall/GMB/BP_PS.BP_PS_C"))
        (for _array_element _outactors
          (Default|UpdateResutlt _array_element))))))

(fn ChecktoReady
  (bind _outactors (Actor|GetAllActorsOfClass "/Game/FootBall/GMB/BP_PC.BP_PC_C"))
  (return (>= (Utilities|Array|Length _outactors) 2)))