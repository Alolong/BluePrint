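; Player state for the football game mode, holding each player's team, nickname, goal count, stamina (SP) and running flag.
; Setters change these replicated values, and RepNotifies for team, nickname, goals and SP fire event dispatchers.
; On BeginPlay it fills SP and registers itself with the first player controller's HUD for binding.
; Running requires remaining SP; the running RepNotify is empty and UpdateResutlt only casts the game state.
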(event EventBeginPlay
  (Variables|Default|SetCurSP (Variables|Default|GetMaxSP))
  ;[0.15 0.15 0.15 0.5] 플레이어스테이트 생성시마다 바인드를 걸어줌
  (bind _asbp_hud (Utilities|Casting|CastToBP_Hud (HUD|GetHUD (Game|GetPlayerController 0))))
  (Default|BindPS _asbp_hud self))

(event EventTick
  (params (DeltaSeconds :type Float%20%28single-precision%29)))

(fn ConstructionScript)

(fn UpdateTeam
  (params (Team :type EN_Team%20Enum :default "NewEnumerator0"))
  (Variables|Default|SetTeam Team))

(fn OnRepTeam
  (Default|CallDSUpdateTeam (Variables|Default|GetTeam)))

(fn ChangeNickName
  (params (NickName :type String))
  (Variables|Default|SetNickName NickName))

(fn OnRepNickName
  (Default|CallDSChangeNickName (Variables|Default|GetNickName)))

(fn AddGoal
  (Variables|Default|SetGoal (+ (Variables|Default|GetGoal) 1)))

(fn OnRepGoal
  (Default|CallDSUpdateGoal (Variables|Default|GetGoal)))

(fn UpdateResutlt
  (Utilities|Casting|CastToBP_GSB (Game|GetGameState)))

(fn UseSP
  (params (UseValue :type Float%20%28double-precision%29))
  (Variables|Default|SetCurSP (Math|Float|Clamp(Float) (- (Variables|Default|GetCurSP) UseValue) 0.0 (Variables|Default|GetMaxSP))))

(fn OnRepCurSP
  (Default|CallDSUpdateSP (Variables|Default|GetCurSP) (Variables|Default|GetMaxSP)))

(fn IsCanRun
  (return (> (Variables|Default|GetCurSP) 0.0)))

(fn SetRun
  (params (IsCanRun :type Boolean))
  ;[0.15 0.15 0.15 0.5] 예외처리
  (if (and IsCanRun (CallFunction|IsCanRun))
    (Variables|Default|SetIsRunning true)
    (else
      (Variables|Default|SetIsRunning false))))

(fn OnRepIsRunning)